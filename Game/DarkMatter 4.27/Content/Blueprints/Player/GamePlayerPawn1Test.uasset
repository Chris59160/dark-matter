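; Test player pawn that snaps its mesh to the first tagged spawn actor on BeginPlay and enables tick when an intro timeline finishes.
; Releasing Q runs a custom Destroy, which spawns an explosion with sound and hides the mesh without removing the actor.
; A helper offsets the mesh by the main camera's frame-to-frame movement with sweep, but nothing here calls it and Tick is empty.
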(event EventBeginPlay
  (Input|EnableInput (Game|GetPlayerController 0))
  (CallFunction|SetInitialLocation)
  (Timeline|Timeline_0 Play
    (:Finished
      (Actor|Tick|SetActorTickEnabled true))))

(event Collision|EventActorBeginOverlap
  (params (OtherActor :type Actor%20Object%20Reference)))

(event EventTick
  (params (DeltaSeconds :type Float%20%28single-precision%29)))

(event Input|KeyboardEvents|Q
  (params (Key :type Key%20Structure :default "None"))
  (:Released
    (CallFunction|Destroy)))

(fn ConstructionScript)

(fn Destroy
  (bind _staticmesh (Variables|Default|GetStaticMesh))
  (Development|PrintString "Destroy GameplayerPawn")
  (Game|SpawnActorfromClass "/Game/Blueprints/ExplosionBlueprint.ExplosionBlueprint_C" (Math|Transform|MakeTransform (Transformation|GetWorldLocation _staticmesh) "0, 0, 0" "1,1,1") "Undefined" 0 0)
  (Audio|PlaySoundatLocation "/Game/Sounds/fxs/explosion_asteroid.explosion_asteroid" (Transformation|GetWorldLocation _staticmesh) "0, 0, 0" 1.0 1.0 0.0 0 0 0)
  (Rendering|SetVisibility (Variables|Default|GetStaticMesh) false false))

(fn UpdateActorLocationfromCamera
  (bind _main_camera (Variables|Default|GetMain%20Camera))
  (bind _rootcomponent (Variables|/Script/Engine.Actor|GetRootComponent _main_camera))
  (bind _returnvalue (Transformation|GetWorldLocation _rootcomponent))
  (Development|PrintString "Update Actor Location")
  (if (Utilities|IsValid (Variables|Default|GetMain%20Camera))
    (if (Variables|Default|GetCamera%20Previous%20Location%20Setted)
      (bind _output_get (LocalVariables|SetCamera%20Current%20Location _returnvalue))
      (bind _newparam (CallFunction|GetRootMove self))
      (Transformation|AddLocalOffset _newparam (- _output_get (Variables|Default|GetCamera%20Previous%20Location)) true false)
      (Variables|Default|SetCamera%20Previous%20Location (LocalVariables|GetCamera%20Current%20Location))
      (else
        (Variables|Default|SetCamera%20Previous%20Location _returnvalue)
        (Variables|Default|SetCamera%20Previous%20Location%20Setted true)))))

(fn SetInitialLocation
  (bind _outactors (Actor|GetAllActorswithTag "CONNARD"))
  (if (>= (Utilities|Array|Length _outactors) 1)
    (bind _newparam (CallFunction|GetRootMove))
    (Transformation|SetWorldLocation _newparam (Transformation|GetWorldLocation (Variables|/Script/Engine.Actor|GetRootComponent (Utilities|Array|Get(acopy) _outactors))) true false)
    (Development|PrintString (Utilities|String|Append "Location:" (Utilities|String|ToString(Vector) (Transformation|GetWorldLocation (Variables|/Script/Engine.Actor|GetRootComponent (Utilities|Array|Get(acopy) _outactors))))))))

(fn GetRootMove
  (return (Variables|Default|GetStaticMesh)))