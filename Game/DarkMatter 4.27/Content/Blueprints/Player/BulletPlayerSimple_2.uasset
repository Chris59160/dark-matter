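; Player bullet actor that damages enemies on impact and then destroys itself.
; A mesh hit event runs ProcessHitCollision, which only acts on actors carrying a TypeEnemy component.
; Damage is the bullet's own Attack minus the target's Defense, both read from AttackDefenceComponents, and is passed to the target's TakeDamageComponent.
; Every hit prints a debug string and destroys the bullet, whatever it struck.
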(event OnComponentHit(StaticMesh)
  (params (HitComponent :type Primitive%20Component%20Object%20Reference) (OtherActor :type Actor%20Object%20Reference) (OtherComp :type Primitive%20Component%20Object%20Reference) (NormalImpulse :type Vector :default "0, 0, 0") (Hit :type Hit%20Result%20Structure%20%28by%20ref%29))
  (CallFunction|ProcessHitCollision OtherActor)
  (Development|PrintString "Bullet Hit")
  (Actor|DestroyActor))

(event EventBeginPlay)

(event Collision|EventActorBeginOverlap
  (params (OtherActor :type Actor%20Object%20Reference)))

(event EventTick
  (params (DeltaSeconds :type Float%20%28single-precision%29)))

(fn ConstructionScript)

(fn ProcessHitCollision
  (params (Other :type Actor%20Object%20Reference))
  (LocalVariables|SetOther%20Actor Other)
  (if (Utilities|IsValid (Actor|GetComponentbyClass Other "/Game/Components/Type/TypeEnemy.TypeEnemy_C"))
    (bind _defense (CallFunction|GetActorAttackDefense (LocalVariables|GetOther%20Actor)))
    (bind _attack (CallFunction|GetActorAttackDefense self))
    (Default|Damage (Actor|GetComponentbyClass (LocalVariables|GetOther%20Actor) "/Game/Components/TakeDamageComponent.TakeDamageComponent_C") (- _attack _defense))))

(fn GetActorAttackDefense
  (params (Actor :type Actor%20Object%20Reference))
  (bind _returnvalue (Actor|GetComponentbyClass Actor "/Game/Components/AttackDefenceComponent.AttackDefenceComponent_C"))
  (return (Variables|/Game/Components/AttackDefenceComponent.AttackDefenceComponent_C|GetAttack _returnvalue) (Variables|/Game/Components/AttackDefenceComponent.AttackDefenceComponent_C|GetDefence _returnvalue)))