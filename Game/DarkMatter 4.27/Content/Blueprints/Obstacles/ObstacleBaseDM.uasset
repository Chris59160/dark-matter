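; Base destructible obstacle that spins at a random rate, set at BeginPlay within per-axis min/max bounds.
; When its HealthComponent empties, radius damage shatters the Destructible and a timeline drives a scalar on its dynamic material, though the parameter name is None.
; The explosion spawn inheriting the spin, score award through the Stats actor and actor destruction are disconnected, so they never run.
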(event Custom|Dead%20Triggered
  ;[1 1 1] Explode the Destructible
  (Class|DestructibleComponent|ApplyRadiusDamage (Variables|Default|GetDestructible) 1e+04 (Variables|Default|GetHurt%20Origin) 1.2e+02 5e+02 true)
  (Development|PrintString "DEAD")
  (bind _alpha_out (Timeline|Timeline_0 PlayFromStart)
    (:Update
      (Rendering|Material|SetScalarParameterValue (Variables|Default|Getmaterial%20instance) "None" _alpha_out :!class /Script/Engine.MaterialInstanceDynamic))))

(event EventBeginPlay
  (EventDispatchers|BindEventtoEmpty (Variables|Default|GetHealthComponent) (delegate Custom|Dead%20Triggered))
  (bind _returnvalue (Rendering|Material|CreateDynamicMaterialInstance (Variables|Default|GetDestructible) 0 0 "None" :!class /Script/Engine.PrimitiveComponent))
  (Variables|Default|Setmaterial%20instance _returnvalue)
  (CallFunction|InitiliaseRotatingRate))

(event EventTick
  (params (DeltaSeconds :type Float%20%28single-precision%29)))

(fn ConstructionScript)

(fn AddScore
  (bind _returnvalue (Actor|GetActorOfClass "/Game/Blueprints/Utils/Stats.Stats_C"))
  (Default|AddScore (Actor|GetComponentbyClass _returnvalue "/Game/Components/Stats/PlayerScoreComponent.PlayerScoreComponent_C") (Variables|/Game/Components/Stats/ScoreComponent.ScoreComponent_C|Getscore (Variables|Default|GetScoreComponent))))

(fn InitiliaseRotatingRate
  (bind _rotatingratemininum (Variables|Default|GetRotatingRateMininum))
  (bind _rotatingratemaximum (Variables|Default|GetRotatingRateMaximum))
  (Variables|/Script/Engine.RotatingMovementComponent|SetRotationRate (Variables|Default|GetRotatingMovement) (Math|Rotator|MakeRotator (Math|Random|RandomFloatinRange (.x _rotatingratemininum) (.x _rotatingratemaximum)) (Math|Random|RandomFloatinRange (.y _rotatingratemininum) (.y _rotatingratemaximum)) (Math|Random|RandomFloatinRange (.z _rotatingratemininum) (.z _rotatingratemaximum)))))