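; Small destructible-mesh obstacle Blueprint that extends a parent obstacle class.
; On BeginPlay it sets a maximum rotating rate, then runs the parent's BeginPlay.
; Destructible component hits store the impact location as HurtOrigin, and fractures only print a debug message.
; A radius-damage call meant to shatter the mesh is left disconnected, so this Blueprint never applies damage itself.
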(event OnComponentHit(Destructible)
  (params (HitComponent :type Primitive%20Component%20Object%20Reference) (OtherActor :type Actor%20Object%20Reference) (OtherComp :type Primitive%20Component%20Object%20Reference) (NormalImpulse :type Vector :default "0, 0, 0") (Hit :type Hit%20Result%20Structure%20%28by%20ref%29))
  (Variables|Default|SetHurt%20Origin (.location Hit)))

(event OnComponentFracture(Destructible)
  (params (HitPoint :type Vector%20%28by%20ref%29 :default "0, 0, 0") (HitDirection :type Vector%20%28by%20ref%29 :default "0, 0, 0"))
  (Development|PrintString "FRACTURE STARTED"))

(event EventBeginPlay
  (Variables|Default|SetRotatingRateMaximum "10.000000,10.000000,10.000000")
  (|CallParentFunction))

(event Collision|EventActorBeginOverlap
  (params (OtherActor :type Actor%20Object%20Reference)))

(event EventTick
  (params (DeltaSeconds :type Float%20%28single-precision%29))
  (|CallParentFunction DeltaSeconds) ; This node is disabled and will not be called.\nDrag off pins to build functionality.
)

(fn ConstructionScript
  (|CallParentFunction))