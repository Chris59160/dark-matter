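; ObstacleBase is a destructible obstacle Actor that halts the CameraMain actor's velocity while something overlaps its box.
; BoxOverlap begin and end events find CameraMain and call SetToZero or Reset on its VelocityComponent, without checking which actor overlapped.
; When HealthComponent signals death, it spawns an explosion at the root's location and scale, then destroys itself.
; Hit and overlap events also print debug strings.
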(event OnComponentBeginOverlap(BoxOverlap)
  (params (OverlappedComponent :type Primitive%20Component%20Object%20Reference) (OtherActor :type Actor%20Object%20Reference) (OtherComp :type Primitive%20Component%20Object%20Reference) (OtherBodyIndex :type Integer) (bFromSweep :type Boolean) (SweepResult :type Hit%20Result%20Structure%20%28by%20ref%29))
  (Development|PrintString "Overlap Obstable Start")
  (bind _returnvalue (Actor|GetActorOfClass "/Game/Blueprints/Cameras/CameraMain.CameraMain_C"))
  (Default|SettoZero (Actor|GetComponentbyClass _returnvalue "/Game/Components/VelocityComponent.VelocityComponent_C")))

(event OnComponentHit(BoxHit)
  (params (HitComponent :type Primitive%20Component%20Object%20Reference) (OtherActor :type Actor%20Object%20Reference) (OtherComp :type Primitive%20Component%20Object%20Reference) (NormalImpulse :type Vector :default "0, 0, 0") (Hit :type Hit%20Result%20Structure%20%28by%20ref%29))
  (Development|PrintString "Hit OBstacleBase"))

(event OnComponentEndOverlap(BoxOverlap)
  (params (OverlappedComponent :type Primitive%20Component%20Object%20Reference) (OtherActor :type Actor%20Object%20Reference) (OtherComp :type Primitive%20Component%20Object%20Reference) (OtherBodyIndex :type Integer))
  (Development|PrintString "Overlap Obstacle End")
  (bind _returnvalue (Actor|GetActorOfClass "/Game/Blueprints/Cameras/CameraMain.CameraMain_C"))
  (Default|Reset (Actor|GetComponentbyClass _returnvalue "/Game/Components/VelocityComponent.VelocityComponent_C")))

(event OnComponentHit(StaticMesh)
  (params (HitComponent :type Primitive%20Component%20Object%20Reference) (OtherActor :type Actor%20Object%20Reference) (OtherComp :type Primitive%20Component%20Object%20Reference) (NormalImpulse :type Vector :default "0, 0, 0") (Hit :type Hit%20Result%20Structure%20%28by%20ref%29))
  (Development|PrintString "Obstacle Mesh Hit"))

(event Custom|Dead%20Triggered
  (bind _defaultsceneroot (Variables|Default|GetDefaultSceneRoot))
  (Game|SpawnActorfromClass "/Game/Blueprints/ExplosionBlueprint.ExplosionBlueprint_C" (Math|Transform|MakeTransform (Transformation|GetWorldLocation _defaultsceneroot) "0, 0, 0" (Transformation|GetWorldScale _defaultsceneroot)) "AlwaysSpawn" 0 0)
  (Actor|DestroyActor))

(event EventBeginPlay
  (EventDispatchers|BindEventtoDead (Variables|Default|GetHealthComponent) (delegate Custom|Dead%20Triggered)))

(event EventTick
  (params (DeltaSeconds :type Float%20%28single-precision%29)))

(fn ConstructionScript)