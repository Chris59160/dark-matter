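; Player pawn for a shooter, delegating movement, tilt, firing, health, stamina and slow-down to components.
; BeginPlay sets up shots, HUD and start position, then enables tick after a timeline so the mesh follows the main camera's movement delta with sweep.
; Input drives movement, single-shot fire, FOV zoom and stamina-limited sprint; death spawns an explosion.
; Attack-minus-defence collision damage is unwired, and the double shot is initialised but never fired.
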(event OnComponentHit(StaticMesh)
  (params (HitComponent :type Primitive%20Component%20Object%20Reference) (OtherActor :type Actor%20Object%20Reference) (OtherComp :type Primitive%20Component%20Object%20Reference) (NormalImpulse :type Vector :default "0, 0, 0") (Hit :type Hit%20Result%20Structure%20%28by%20ref%29)))

(event OnComponentBeginOverlap(StaticMesh)
  (params (OverlappedComponent :type Primitive%20Component%20Object%20Reference) (OtherActor :type Actor%20Object%20Reference) (OtherComp :type Primitive%20Component%20Object%20Reference) (OtherBodyIndex :type Integer) (bFromSweep :type Boolean) (SweepResult :type Hit%20Result%20Structure%20%28by%20ref%29))
  (Development|PrintString "Overlapma ass"))

(event Custom|Dead
  (CallFunction|Destroy))

(event Custom|Stamina%20Drained
  (Variables|/Game/Components/VelocityComponent.VelocityComponent_C|SetVelocity (Variables|Default|GetVelocityComponent) 5e+02))

(event EventBeginPlay
  (Input|EnableInput (Game|GetPlayerController 0))
  (CallFunction|InitShotComponents)
  ;[1 1 1] Draw HUD on Screen
  (CallFunction|DrawHud)
  (EventDispatchers|BindEventtoDrained (Variables|Default|GetStaminaComponent) (delegate Custom|Stamina%20Drained))
  (EventDispatchers|BindEventtoDead (Variables|Default|GetHealthComponent) (delegate Custom|Dead))
  (CallFunction|SetMainCamera)
  (CallFunction|SetInitialLocation)
  (Timeline|Timeline_0 Play
    (:Finished
      (Actor|Tick|SetActorTickEnabled true)
      (Variables|/Game/Components/player/PlayerTiltComponent.PlayerTiltComponent_C|SetStatic%20Mesh (Variables|Default|GetPlayerTiltComponent) (Variables|Default|GetStaticMesh1)))))

(event Collision|EventActorBeginOverlap
  (params (OtherActor :type Actor%20Object%20Reference)))

(event EventTick
  (params (DeltaSeconds :type Float%20%28single-precision%29))
  (CallFunction|UpdateActorLocationfromCamera))

(event Input|ActionEvents|InputActionFireLight
  (params (Key :type Key%20Structure :default "None"))
  (bind _singleshotdirectioncomponent (Variables|Default|GetSingleShotDirectionComponent))
  ;[1 1 1] Fire Light Bullet
  (:Pressed
    (Variables|/Game/Components/ShotDirectionComponent.ShotDirectionComponent_C|SetFireShotReleased _singleshotdirectioncomponent false)
    (Default|StartShooting (Variables|Default|GetSingleShotDirectionComponent)))
  (:Released
    (Variables|/Game/Components/ShotDirectionComponent.ShotDirectionComponent_C|SetFireShotReleased _singleshotdirectioncomponent true)))

(event Input|ActionEvents|InputActionSprint
  (params (Key :type Key%20Structure :default "None"))
  (bind _staminacomponent (Variables|Default|GetStaminaComponent))
  (bind _velocitycomponent (Variables|Default|GetVelocityComponent))
  ;[1 1 1] Sprint Flow
  (:Pressed
    (Default|Start _staminacomponent)
    (Variables|/Game/Components/VelocityComponent.VelocityComponent_C|SetVelocity _velocitycomponent 1e+03))
  (:Released
    (Default|Stop _staminacomponent)
    (Variables|/Game/Components/VelocityComponent.VelocityComponent_C|SetVelocity _velocitycomponent 5e+02)))

(event Input|ActionEvents|InputActionZoom
  (params (Key :type Key%20Structure :default "None"))
  ;[1 1 1] Zoom In Out In Front of the Camera
  (:Pressed
    (bind _zoom (Timeline|Zoom%20In%20Out Play)
      (:Update
        (bind _ascamera_actor (Utilities|Casting|CastToCameraActor (Pawn|GetViewTarget (Game|GetPlayerController 0))))
        (Camera|SetFieldOfView (Variables|/Script/Engine.CameraActor|GetCameraComponent _ascamera_actor) _zoom))))
  (:Released
    (Timeline|Zoom%20In%20Out Reverse)))

(event Input|ActionEvents|InputActionTriggerSlowDown
  (params (Key :type Key%20Structure :default "None"))
  ;[1 1 1] Slow Down Manual Trigger for Debug
  (:Released
    (Default|Start (Variables|Default|GetSlowDownComponent))))

(event Input|AxisEvents|InputAxisMoveLateral
  (params (AxisValue :type Float%20%28single-precision%29))
  ;[1 1 1] Move Lateral managed by PlayerMovement
  (Default|MoveLateral (Variables|Default|GetPlayerMovement) AxisValue)
  (Default|ProcessAxis (Variables|Default|GetPlayerTiltComponent) AxisValue))

(event Input|AxisEvents|InputAxisMoveForward
  (params (AxisValue :type Float%20%28single-precision%29))
  ;[1 1 1] Move Forward managed by PlayerMovement
  (Default|MoveForward (Variables|Default|GetPlayerMovement) AxisValue))

(fn ConstructionScript)

(fn InitShotComponents
  (Default|SetLocationComponent (Variables|Default|GetSingleShotDirectionComponent) (Variables|Default|GetSingletBulletSpawnLocation))
  (Default|SetLocationComponent (Variables|Default|GetDoubleShotDirectionComponent) (Variables|Default|GetLeftBulletSpawnLocation) (Variables|Default|GetRightBulletSpawnLocation)))

(fn DrawHud
  (bind _returnvalue (UserInterface|CreateWidget "/Game/UI/HUD.HUD_C"))
  (UserInterface|Viewport|AddtoViewport _returnvalue 0))

(fn Destroy
  (bind _staticmesh (Variables|Default|GetStaticMesh))
  (Game|SpawnActorfromClass "/Game/Blueprints/ExplosionBlueprint.ExplosionBlueprint_C" (Math|Transform|MakeTransform (Transformation|GetWorldLocation _staticmesh) "0, 0, 0" "1,1,1") "Undefined" 0 0)
  (Audio|PlaySoundatLocation "/Game/Sounds/fxs/explosion_asteroid.explosion_asteroid" (Transformation|GetWorldLocation _staticmesh) "0, 0, 0" 1.0 1.0 0.0 0 0 0)
  (Actor|DestroyActor))

(fn ProcessHitCollision
  (params (Other :type Actor%20Object%20Reference))
  (LocalVariables|SetOther%20Actor Other)
  (if (Utilities|IsValid (Actor|GetComponentbyClass Other "/Game/Components/Type/TypeEnemy.TypeEnemy_C"))
    (bind (_attack _defense) (CallFunction|GetActorAttackDefense (LocalVariables|GetOther%20Actor)))
    (bind (_attack_2 _defense_2) (CallFunction|GetActorAttackDefense self))
    (Default|Damage (Actor|GetComponentbyClass (LocalVariables|GetOther%20Actor) "/Game/Components/TakeDamageComponent.TakeDamageComponent_C") (- _attack_2 _defense))
    (Default|Damage (Actor|GetComponentbyClass "/Game/Components/TakeDamageComponent.TakeDamageComponent_C") (- _attack _defense_2))))

(fn GetActorAttackDefense
  (params (Actor :type Actor%20Object%20Reference))
  (bind _returnvalue (Actor|GetComponentbyClass Actor "/Game/Components/AttackDefenceComponent.AttackDefenceComponent_C"))
  (return (Variables|/Game/Components/AttackDefenceComponent.AttackDefenceComponent_C|GetAttack _returnvalue) (Variables|/Game/Components/AttackDefenceComponent.AttackDefenceComponent_C|GetDefence _returnvalue)))

(fn UpdateActorLocationfromCamera
  (bind _main_camera (Variables|Default|GetMain%20Camera))
  (bind _rootcomponent (Variables|/Script/Engine.Actor|GetRootComponent _main_camera))
  (bind _returnvalue (Transformation|GetWorldLocation _rootcomponent))
  (if (Utilities|IsValid (Variables|Default|GetMain%20Camera))
    (if (Variables|Default|GetCamera%20Previous%20Location%20Setted)
      (bind _output_get (LocalVariables|SetCamera%20Current%20Location _returnvalue))
      (bind _newparam (CallFunction|GetRootMove self))
      (Transformation|AddLocalOffset _newparam (- _output_get (Variables|Default|GetCamera%20Previous%20Location)) true false)
      (Variables|Default|SetCamera%20Previous%20Location (LocalVariables|GetCamera%20Current%20Location))
      (else
        (Variables|Default|SetCamera%20Previous%20Location _returnvalue)
        (Variables|Default|SetCamera%20Previous%20Location%20Setted true)))))

(fn SetMainCamera
  (bind _returnvalue (Actor|GetActorOfClass "/Game/Blueprints/Cameras/CameraMain.CameraMain_C"))
  (if (Utilities|IsValid _returnvalue)
    (Variables|Default|SetMain%20Camera _returnvalue)))

(fn SetInitialLocation
  (bind _outactors (Actor|GetAllActorswithTag "CONNARD"))
  (if (>= (Utilities|Array|Length _outactors) 1)
    (bind _newparam (CallFunction|GetRootMove))
    (Transformation|SetWorldLocation _newparam (Transformation|GetWorldLocation (Variables|/Script/Engine.Actor|GetRootComponent (Utilities|Array|Get(acopy) _outactors))) true false)
    (Development|PrintString (Utilities|String|Append "Location:" (Utilities|String|ToString(Vector) (Transformation|GetWorldLocation (Variables|/Script/Engine.Actor|GetRootComponent (Utilities|Array|Get(acopy) _outactors))))))))

(fn GetRootMove
  (return (Variables|Default|GetStaticMesh)))