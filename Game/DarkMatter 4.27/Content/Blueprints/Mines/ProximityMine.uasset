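; A proximity mine actor that reacts to actors entering and leaving its sphere.
; Sphere begin and end overlaps are forwarded to a MineProximityComponent, which holds the trigger type and handles the overlap logic.
; On BeginPlay it enables player input and targets characters; number keys 0–2 switch the trigger type between enemy, player and character, apparently for testing.
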(event OnComponentEndOverlap(Sphere)
  (params (OverlappedComponent :type Primitive%20Component%20Object%20Reference) (OtherActor :type Actor%20Object%20Reference) (OtherComp :type Primitive%20Component%20Object%20Reference) (OtherBodyIndex :type Integer))
  (Default|StopOverlap (Variables|Default|GetMineProximityComponent) OtherActor))

(event OnComponentBeginOverlap(Sphere)
  (params (OverlappedComponent :type Primitive%20Component%20Object%20Reference) (OtherActor :type Actor%20Object%20Reference) (OtherComp :type Primitive%20Component%20Object%20Reference) (OtherBodyIndex :type Integer) (bFromSweep :type Boolean) (SweepResult :type Hit%20Result%20Structure%20%28by%20ref%29))
  (Default|StartOverlap (Variables|Default|GetMineProximityComponent) OtherActor))

(event EventBeginPlay
  (Input|EnableInput (Game|GetPlayerController 0))
  (Variables|/Game/Components/Mines/MineProximityComponent.MineProximityComponent_C|SetTriggerType (Variables|Default|GetMineProximityComponent) "/Game/Components/Type/TypeCharacter.TypeCharacter_C"))

(event Collision|EventActorBeginOverlap
  (params (OtherActor :type Actor%20Object%20Reference)))

(event EventTick
  (params (DeltaSeconds :type Float%20%28single-precision%29)))

(event Input|KeyboardEvents|0
  (params (Key :type Key%20Structure :default "None"))
  (:Released
    (Variables|/Game/Components/Mines/MineProximityComponent.MineProximityComponent_C|SetTriggerType (Variables|Default|GetMineProximityComponent) "/Game/Components/Type/TypeEnemy.TypeEnemy_C")))

(event Input|KeyboardEvents|1
  (params (Key :type Key%20Structure :default "None"))
  (:Released
    (Variables|/Game/Components/Mines/MineProximityComponent.MineProximityComponent_C|SetTriggerType (Variables|Default|GetMineProximityComponent) "/Game/Components/Type/TypePlayer.TypePlayer_C")))

(event Input|KeyboardEvents|2
  (params (Key :type Key%20Structure :default "None"))
  (:Released
    (Variables|/Game/Components/Mines/MineProximityComponent.MineProximityComponent_C|SetTriggerType (Variables|Default|GetMineProximityComponent) "/Game/Components/Type/TypeCharacter.TypeCharacter_C")))

(fn ConstructionScript)