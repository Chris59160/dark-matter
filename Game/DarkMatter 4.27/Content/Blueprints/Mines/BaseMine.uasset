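; Base mine actor Blueprint that forwards proximity overlaps to a MineComponent and blinks its mesh when the mine is triggered.
; Sphere begin and end overlap events pass the other actor to the component's StartOverlap and StopOverlap.
; On BeginPlay it creates a dynamic material instance on the static mesh and binds to the component's triggered event.
; When triggered, a timeline drives the material's Factor parameter to produce the blink.
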(event OnComponentBeginOverlap(Sphere)
  (params (OverlappedComponent :type Primitive%20Component%20Object%20Reference) (OtherActor :type Actor%20Object%20Reference) (OtherComp :type Primitive%20Component%20Object%20Reference) (OtherBodyIndex :type Integer) (bFromSweep :type Boolean) (SweepResult :type Hit%20Result%20Structure%20%28by%20ref%29))
  (Default|StartOverlap (Actor|GetComponentbyClass "/Game/Components/Mines/MineComponent.MineComponent_C") OtherActor))

(event OnComponentEndOverlap(Sphere)
  (params (OverlappedComponent :type Primitive%20Component%20Object%20Reference) (OtherActor :type Actor%20Object%20Reference) (OtherComp :type Primitive%20Component%20Object%20Reference) (OtherBodyIndex :type Integer))
  (Default|StopOverlap (Actor|GetComponentbyClass "/Game/Components/Mines/MineComponent.MineComponent_C") OtherActor))

(event Custom|MineTriggered
  (bind _material_parameter (Timeline|TimelineBlinking PlayFromStart)
    (:Update
      (Rendering|Material|SetScalarParameterValue (Variables|Default|GetMaterialInstance) "Factor" _material_parameter :!class /Script/Engine.MaterialInstanceDynamic))))

(event EventBeginPlay
  (CallFunction|CreateMaterialInstance)
  (EventDispatchers|BindEventtoTriggered (Actor|GetComponentbyClass "/Game/Components/Mines/MineComponent.MineComponent_C") (delegate Custom|MineTriggered)))

(event Collision|EventActorBeginOverlap
  (params (OtherActor :type Actor%20Object%20Reference)))

(event EventTick
  (params (DeltaSeconds :type Float%20%28single-precision%29)))

(fn ConstructionScript)

(fn CreateMaterialInstance
  (bind _returnvalue (Rendering|Material|CreateDynamicMaterialInstance (Variables|Default|GetStaticMesh) 0 0 "None" :!class /Script/Engine.PrimitiveComponent))
  (Variables|Default|SetMaterialInstance _returnvalue))