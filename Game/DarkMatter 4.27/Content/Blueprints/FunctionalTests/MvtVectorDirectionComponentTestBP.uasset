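; Functional test that checks an actor's MvtVectorDirectionComponent moves it in the expected direction.
; On start it sets the component's direction, records the actor's location and starts a success timer.
; Each tick it compares X with the previous location and fails if X increases, so stationary or decreasing X passes.
; Only the X axis is checked, whatever direction is configured.
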(event EventPrepareTest)

(event EventStartTest
  (bind _actor (Variables|Default|GetActor))
  (Utilities|Time|SetTimerbyFunctionName 0 "FinishEventSuccess" (Variables|Default|GetTimeValidateTest))
  (Default|SetDirection (Actor|GetComponentbyClass _actor "/Game/Components/MvtVectorDirectionComponent.MvtVectorDirectionComponent_C") (Variables|Default|GetMovementDirection))
  (Variables|Default|SetPreviousLocation (Transformation|GetActorLocation _actor)))

(event EventTick
  (params (DeltaSeconds :type Float%20%28single-precision%29))
  (if (>= (.x (Variables|Default|GetPreviousLocation)) (.x (Transformation|GetActorLocation (Variables|Default|GetActor))))
    (Variables|Default|SetPreviousLocation (Transformation|GetActorLocation (Variables|Default|GetActor)))
    (else
      (Class|FunctionalTest|FinishTest "Failed" "The Location of the object isn't being updated correctly"))))

(fn ConstructionScript)

(fn FinishEventSuccess
  (Class|FunctionalTest|FinishTest "Succeeded" "Mouvement Direction Test Successfull"))