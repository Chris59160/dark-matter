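; Functional test that checks the player pawn's StaminaComponent drains and then restores correctly.
; Preparation seeds the component's value and default; starting the test binds its Drained and Restored events and starts it.
; Each tick asserts the value never moves against the current phase, failing otherwise.
; The Drained event stops the component to switch to the restore phase, and the Restored event finishes the test as succeeded.
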(event Custom|ValueEmpty_Event
  (bind _returnvalue (Game|Player|GetPlayerPawn 0))
  (bind _returnvalue_2 (Actor|GetComponentbyClass _returnvalue "/Game/Components/StaminaComponent.StaminaComponent_C"))
  (Variables|Default|SetIs%20Draining false)
  (Variables|Default|SetCurrent%20Value (Variables|/Game/Components/RestoreDrainComponent.RestoreDrainComponent_C|GetValue _returnvalue_2))
  (Default|Stop _returnvalue_2)
  (Class|FunctionalTest|LogMessage "Draining is finished, now restoring"))

(event Custom|ValueRestored_Event
  (Class|FunctionalTest|FinishTest "Succeeded" "RestoreDrain Stamina Worked"))

(event EventPrepareTest
  (CallFunction|InitialiseTest)
  (Variables|Default|SetCurrent%20Value (Variables|Default|GetInitial%20Value))
  (Class|FunctionalTest|LogMessage "Initialisation Done"))

(event EventStartTest
  (bind _returnvalue (Game|Player|GetPlayerPawn 0))
  (bind _returnvalue_2 (Actor|GetComponentbyClass _returnvalue "/Game/Components/StaminaComponent.StaminaComponent_C"))
  (CallFunction|StartTest)
  (EventDispatchers|BindEventtoDrained _returnvalue_2 (delegate Custom|ValueEmpty_Event))
  (EventDispatchers|BindEventtoRestored _returnvalue_2 (delegate Custom|ValueRestored_Event))
  (Class|FunctionalTest|LogMessage "Started Draining"))

(event EventTick
  (params (DeltaSeconds :type Float%20%28single-precision%29))
  (if (Variables|Default|GetIs%20Draining)
    (CallFunction|CheckDraining)
    (else
      (CallFunction|CheckRestoring)))
  (CallFunction|LogCurrentValue))

(fn ConstructionScript)

(fn InitialiseTest
  (bind _returnvalue (Game|Player|GetPlayerPawn 0))
  (bind _initial_value (Variables|Default|GetInitial%20Value))
  (bind _returnvalue_2 (Actor|GetComponentbyClass _returnvalue "/Game/Components/StaminaComponent.StaminaComponent_C"))
  (bind _returnvalue_3 (Class|FunctionalTest|AssertIsValid _returnvalue_2 "Can't find Stamina Component"))
  (if _returnvalue_3
    (Variables|/Game/Components/RestoreDrainComponent.RestoreDrainComponent_C|SetValue _returnvalue_2 _initial_value)
    (bind _output_get (Variables|/Game/Components/RestoreDrainComponent.RestoreDrainComponent_C|SetDefault%20Value _returnvalue_2 _initial_value))
    (Class|FunctionalTest|LogMessage (Utilities|String|Append "RestroDrainComponent Test Start: " (Utilities|String|ToString(Float) _output_get)))))

(fn StartTest
  (Default|Start (Actor|GetComponentbyClass (Game|Player|GetPlayerPawn 0) "/Game/Components/StaminaComponent.StaminaComponent_C")))

(fn CheckDraining
  (bind _returnvalue (Game|Player|GetPlayerPawn 0))
  (bind _returnvalue_2 (Actor|GetComponentbyClass _returnvalue "/Game/Components/StaminaComponent.StaminaComponent_C"))
  (bind _value (Variables|/Game/Components/RestoreDrainComponent.RestoreDrainComponent_C|GetValue _returnvalue_2))
  (bind _returnvalue_3 (Class|FunctionalTest|AssertTrue (<= _value (Variables|Default|GetCurrent%20Value))))
  (if _returnvalue_3
    (Variables|Default|SetCurrent%20Value _value)
    (else
      (Class|FunctionalTest|FinishTest "Failed" "Test Failed"))))

(fn LogCurrentValue
  (Class|FunctionalTest|LogMessage (Utilities|String|Append "CUrrent Value:: " (Utilities|String|ToString(Float) (Variables|Default|GetCurrent%20Value)))))

(fn CheckRestoring
  (bind _returnvalue (Game|Player|GetPlayerPawn 0))
  (bind _returnvalue_2 (Actor|GetComponentbyClass _returnvalue "/Game/Components/StaminaComponent.StaminaComponent_C"))
  (bind _value (Variables|/Game/Components/RestoreDrainComponent.RestoreDrainComponent_C|GetValue _returnvalue_2))
  (bind _returnvalue_3 (Class|FunctionalTest|AssertTrue (>= _value (Variables|Default|GetCurrent%20Value))))
  (if _returnvalue_3
    (Variables|Default|SetCurrent%20Value _value)
    (else
      (Class|FunctionalTest|FinishTest "Failed" "Test Failed"))))