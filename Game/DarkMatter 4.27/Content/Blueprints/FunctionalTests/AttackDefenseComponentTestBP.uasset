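; Functional test that checks add and subtract arithmetic on the Attack and Defence values of the player pawn's AttackDefenceComponent.
; On StartTest, TestAttack runs first and TestDefense follows only if it succeeds.
; Each function resets its stat to an original value, writes the property directly, and asserts the result against expected variables.
; A failed add assertion finishes the test inside the function, while StartTest reports the overall result.
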(event EventPrepareTest)

(event EventStartTest
  (bind _result (CallFunction|TestAttack))
  (if _result
    (bind _result_2 (CallFunction|TestDefense))
    (if _result_2
      (Class|FunctionalTest|FinishTest "Succeeded" "Attack Full Test Passed")
      (else
        (Class|FunctionalTest|FinishTest "Failed" "Attack Full Test Failed")))
    (else
      (Class|FunctionalTest|FinishTest "Failed" "Sub Attack Failed"))))

(event EventTick
  (params (DeltaSeconds :type Float%20%28single-precision%29)))

(fn ConstructionScript)

(fn TestAttack
  (bind _returnvalue (Game|Player|GetPlayerPawn 0))
  (bind _returnvalue_2 (Game|Player|GetPlayerPawn 0))
  (bind _returnvalue_3 (Actor|GetComponentbyClass _returnvalue "/Game/Components/AttackDefenceComponent.AttackDefenceComponent_C"))
  (bind _returnvalue_4 (Actor|GetComponentbyClass _returnvalue_2 "/Game/Components/AttackDefenceComponent.AttackDefenceComponent_C"))
  (bind _output_get (Variables|/Game/Components/AttackDefenceComponent.AttackDefenceComponent_C|SetAttack _returnvalue_4 (LocalVariables|GetoriginalAttack)))
  (bind _output_get_2 (Variables|/Game/Components/AttackDefenceComponent.AttackDefenceComponent_C|SetAttack _returnvalue_4 (+ _output_get (LocalVariables|GetattackToAdd))))
  (bind _returnvalue_5 (Class|FunctionalTest|AssertEqualInt _output_get_2 (LocalVariables|GetattackAfterAddCheckAgainst) "The Check on Add attack failed"))
  (if _returnvalue_5
    (bind _output_get_3 (Variables|/Game/Components/AttackDefenceComponent.AttackDefenceComponent_C|SetAttack _returnvalue_3 (- (Variables|/Game/Components/AttackDefenceComponent.AttackDefenceComponent_C|GetAttack _returnvalue_3) (LocalVariables|GetattackToSub))))
    (bind _returnvalue_6 (Class|FunctionalTest|AssertEqualInt _output_get_3 (LocalVariables|GetattackAfterSubCheckAgainst)))
    (return _returnvalue_6)
    (else
      (Class|FunctionalTest|FinishTest "Failed" "The Attack Add test didn't go through"))))

(fn TestDefense
  (bind _returnvalue (Game|Player|GetPlayerPawn 0))
  (bind _returnvalue_2 (Game|Player|GetPlayerPawn 0))
  (bind _returnvalue_3 (Actor|GetComponentbyClass _returnvalue "/Game/Components/AttackDefenceComponent.AttackDefenceComponent_C"))
  (bind _returnvalue_4 (Actor|GetComponentbyClass _returnvalue_2 "/Game/Components/AttackDefenceComponent.AttackDefenceComponent_C"))
  (bind _output_get (Variables|/Game/Components/AttackDefenceComponent.AttackDefenceComponent_C|SetDefence _returnvalue_4 (LocalVariables|GetoriginalDefense)))
  (bind _output_get_2 (Variables|/Game/Components/AttackDefenceComponent.AttackDefenceComponent_C|SetDefence _returnvalue_4 (+ _output_get (LocalVariables|GetdefenseToAdd))))
  (bind _returnvalue_5 (Class|FunctionalTest|AssertEqualInt _output_get_2 (LocalVariables|GetdefenseAfterAddCheckAgainst) "The Check on Add Sub failed"))
  (if _returnvalue_5
    (bind _output_get_3 (Variables|/Game/Components/AttackDefenceComponent.AttackDefenceComponent_C|SetDefence _returnvalue_3 (- (Variables|/Game/Components/AttackDefenceComponent.AttackDefenceComponent_C|GetDefence _returnvalue_3) (LocalVariables|GetdefenseToSub))))
    (bind _returnvalue_6 (Class|FunctionalTest|AssertEqualInt _output_get_3 (LocalVariables|GetdefenseAfterSubCheckAgainst)))
    (return _returnvalue_6)
    (else
      (Class|FunctionalTest|FinishTest "Failed" "The Defense Add test didn't go through"))))