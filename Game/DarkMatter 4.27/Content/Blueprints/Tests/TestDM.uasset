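; TestDM is a test actor for exercising damage on a Destructible component.
; It enables player input on BeginPlay so that releasing N applies radius damage at the DamageHitLocation variable.
; A component hit on the Destructible also applies radius damage, with larger damage and radius, at the impact location.
; Both triggers print debug messages.
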(event OnComponentHit(Destructible)
  (params (HitComponent :type Primitive%20Component%20Object%20Reference) (OtherActor :type Actor%20Object%20Reference) (OtherComp :type Primitive%20Component%20Object%20Reference) (NormalImpulse :type Vector :default "0, 0, 0") (Hit :type Hit%20Result%20Structure%20%28by%20ref%29))
  (Development|PrintString "Test HIT")
  (Class|DestructibleComponent|ApplyRadiusDamage (Variables|Default|GetDestructible) 1e+04 (.location Hit) 1.2e+02 5e+02 true))

(event EventBeginPlay
  (Input|EnableInput (Game|GetPlayerController 0)))

(event Collision|EventActorBeginOverlap
  (params (OtherActor :type Actor%20Object%20Reference)))

(event EventTick
  (params (DeltaSeconds :type Float%20%28single-precision%29)))

(event Input|KeyboardEvents|N
  (params (Key :type Key%20Structure :default "None"))
  (:Released
    (Development|PrintString "Hello from TestDM")
    (Class|DestructibleComponent|ApplyRadiusDamage (Variables|Default|GetDestructible) 1e+03 (Variables|Default|GetDamage%20Hit%20Location) 5e+01 1e+03 true)))

(fn ConstructionScript)