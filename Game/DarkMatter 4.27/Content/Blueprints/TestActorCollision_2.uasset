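; Test actor for collision, with a static mesh that the player slides along its local X axis using the P and L keys.
; Holding a key runs a looping timer, set to the frame delta at press time, that calls Move Forward or Move Backward until release.
; Only forward movement sweeps for collision; backward movement offsets without sweeping.
; The mesh's hit and begin-overlap events print guitar debug messages.
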(event OnComponentHit(StaticMesh)
  (params (HitComponent :type Primitive%20Component%20Object%20Reference) (OtherActor :type Actor%20Object%20Reference) (OtherComp :type Primitive%20Component%20Object%20Reference) (NormalImpulse :type Vector :default "0, 0, 0") (Hit :type Hit%20Result%20Structure%20%28by%20ref%29))
  (Development|PrintString "Guitar Hit "))

(event OnComponentBeginOverlap(StaticMesh)
  (params (OverlappedComponent :type Primitive%20Component%20Object%20Reference) (OtherActor :type Actor%20Object%20Reference) (OtherComp :type Primitive%20Component%20Object%20Reference) (OtherBodyIndex :type Integer) (bFromSweep :type Boolean) (SweepResult :type Hit%20Result%20Structure%20%28by%20ref%29))
  (Development|PrintString "Guitar OverLap"))

(event Collision|EventActorBeginOverlap
  (params (OtherActor :type Actor%20Object%20Reference)))

(event EventTick
  (params (DeltaSeconds :type Float%20%28single-precision%29)))

(event EventBeginPlay
  (Input|EnableInput (Game|GetPlayerController 0)))

(event Input|KeyboardEvents|P
  (params (Key :type Key%20Structure))
  (:Pressed
    (Utilities|Time|SetTimerbyFunctionName 0 "Move Forward" (Utilities|Time|GetWorldDeltaSeconds) true))
  (:Released
    (Utilities|Time|ClearTimerbyFunctionName 0 "Move Forward")))

(event Input|KeyboardEvents|L
  (params (Key :type Key%20Structure))
  (:Pressed
    (Utilities|Time|SetTimerbyFunctionName 0 "Move Backward" (Utilities|Time|GetWorldDeltaSeconds) true))
  (:Released
    (Utilities|Time|ClearTimerbyFunctionName 0 "Move Backward")))

(fn ConstructionScript)

(fn MoveForward
  (Transformation|AddLocalOffset (Variables|Default|GetStaticMesh) (Math|Vector|MakeVector (* (Utilities|Time|GetWorldDeltaSeconds) 5e+02) 0.0 0.0) true false))

(fn MoveBackward
  (Transformation|AddLocalOffset (Variables|Default|GetStaticMesh) (Math|Vector|MakeVector (* (Utilities|Time|GetWorldDeltaSeconds) -5e+02) 0.0 0.0) false false))