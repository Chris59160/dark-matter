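; CylinderTarget is a moving shooting target that takes two BulletBlueprint hits to destroy.
; Tick moves it along Y at its Speed, with a Delay and FlipFlop reversing direction and toggling the red material every six seconds.
; The first hit turns it red and primes it; the next plays a sound, spawns a small explosion, increments the player pawn's KillCount and destroys it.
; R and N keys manually set or clear the red material.
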(event OnComponentHit(StaticMeshComponent)
  (params (HitComponent :type Primitive%20Component%20Object%20Reference) (OtherActor :type Actor%20Object%20Reference) (OtherComp :type Primitive%20Component%20Object%20Reference) (NormalImpulse :type Vector :default "0, 0, 0") (Hit :type Hit%20Result%20Structure%20%28by%20ref%29))
  (Utilities|Casting|CastToBulletBlueprint OtherActor)
  (if (Variables|Default|GetPrimed)
    (CallFunction|HitPrimed (Transformation|GetWorldLocation (Variables|Debug|GetStaticMeshComponent)))
    (else
      (CallFunction|HitNotPrimed))))

(event Collision|EventActorBeginOverlap
  (params (OtherActor :type Actor%20Object%20Reference)))

(event EventTick
  (params (DeltaSeconds :type Float%20%28single-precision%29))
  (bind _staticmeshcomponent (Variables|Debug|GetStaticMeshComponent))
  (bind _staticmeshcomponent_2 (Variables|Debug|GetStaticMeshComponent))
  (bind _returnvalue (Transformation|GetWorldTransform _staticmeshcomponent))
  (bind (_location _rotation _scale) (Math|Transform|BreakTransform _returnvalue))
  ;[1 1 1] Update transform each frame
  (Transformation|SetActorTransform (Math|Transform|MakeTransform (+ (* (Math|Vector|Normalize (Variables|Default|GetDirection)) (* (Variables|Default|GetSpeed) (Utilities|Time|GetWorldDeltaSeconds))) _location) _rotation _scale))
  ;[1 1 1] Switch direction every 6 seconds
  (Utilities|FlowControl|Delay 6.0)
  (Utilities|FlowControl|FlipFlop
    (:A
      (Variables|Default|SetDirection "0,-10.000000, 0")
      ;[1 1 1] Alternate color
      (Rendering|Material|SetMaterial _staticmeshcomponent_2 0 "/Game/Materials/TargetRed.TargetRed"))
    (:B
      (Variables|Default|SetDirection "0,10.000000, 0")
      (Rendering|Material|SetMaterial _staticmeshcomponent_2 0 0))))

(event EventBeginPlay
  (Input|EnableInput (Game|GetPlayerController 0)))

(event Input|KeyboardEvents|R
  (params (Key :type Key%20Structure))
  (:Released
    (Rendering|Material|SetMaterial (Variables|Debug|GetStaticMeshComponent) 0 "/Game/Materials/TargetRed.TargetRed")
    (Development|PrintString "Set Red")))

(event Input|KeyboardEvents|N
  (params (Key :type Key%20Structure))
  (:Released
    (Rendering|Material|SetMaterial (Variables|Debug|GetStaticMeshComponent) 0 0)
    (Development|PrintString "Set None")))

(fn ConstructionScript)

(fn HitNotPrimed
  (Rendering|Material|SetMaterial (Variables|Debug|GetStaticMeshComponent) 0 "/Game/Materials/TargetRed.TargetRed")
  (Variables|Default|SetPrimed true))

(fn HitPrimed
  (params (Hit%20Location :type Vector%20%28by%20ref%29))
  (Audio|PlaySoundatLocation "/Game/Sounds/fxs/mixkit-cartoon-fart-or-splat-3056.mixkit-cartoon-fart-or-splat-3056" Hit%20Location "0, 0, 0" 1.0 1.0 0.0 0 0 0)
  (Game|SpawnActorfromClass "/Game/Blueprints/ExplosionBlueprint.ExplosionBlueprint_C" (Math|Transform|MakeTransform Hit%20Location "0, 0, 0" "0.200000,0.200000,0.200000") "Undefined" 0 0)
  (bind _asgame_player_pawn (Utilities|Casting|CastToGamePlayerPawn (Game|Player|GetPlayerPawn 0)))
  (Math|Integer|IncrementInt (Variables|/Game/Blueprints/GamePlayerPawn.GamePlayerPawn_C|GetKillCount _asgame_player_pawn)
    (:%20%20
      (Actor|DestroyActor))))