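; Functional test Blueprint that checks integer health arithmetic on the player pawn's HealthComponent.
; On test start it runs an add check, then a subtract check only if the first passes, finishing as succeeded or failed with a message.
; Each check resets Health to an original value, changes the variable directly, and asserts equality against a configured expected result.
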(event EventPrepareTest)

(event EventStartTest
  (Class|FunctionalTest|LogMessage "Character Functional Test")
  (bind _result (CallFunction|TestHealthAdd))
  (if _result
    (bind _result_2 (CallFunction|TestHealthSub))
    (if _result_2
      (Class|FunctionalTest|FinishTest "Succeeded" "Successfull Health Test")
      (else
        (Class|FunctionalTest|FinishTest "Failed" "Failed Subbing Health")))
    (else
      (Class|FunctionalTest|FinishTest "Failed" "Failed Adding Health"))))

(event EventTick
  (params (DeltaSeconds :type Float%20%28single-precision%29)))

(fn ConstructionScript)

(fn TestHealthAdd
  (bind _returnvalue (Game|Player|GetPlayerPawn 0))
  (bind _returnvalue_2 (Actor|GetComponentbyClass _returnvalue "/Game/Components/HealthComponent.HealthComponent_C"))
  (bind _output_get (Variables|/Game/Components/HealthComponent.HealthComponent_C|SetHealth _returnvalue_2 (LocalVariables|GetOriginal%20Health)))
  (bind _output_get_2 (Variables|/Game/Components/HealthComponent.HealthComponent_C|SetHealth _returnvalue_2 (+ _output_get (LocalVariables|GetHealth%20To%20Add))))
  (bind _returnvalue_3 (Class|FunctionalTest|AssertEqualInt _output_get_2 (LocalVariables|GetHealth%20After%20Add)))
  (return _returnvalue_3))

(fn TestHealthSub
  (bind _returnvalue (Game|Player|GetPlayerPawn 0))
  (bind _returnvalue_2 (Actor|GetComponentbyClass _returnvalue "/Game/Components/HealthComponent.HealthComponent_C"))
  (Class|FunctionalTest|LogMessage "In Test Sub Health")
  (bind _output_get (Variables|/Game/Components/HealthComponent.HealthComponent_C|SetHealth _returnvalue_2 (LocalVariables|GetOriginal%20Health)))
  (bind _output_get_2 (Variables|/Game/Components/HealthComponent.HealthComponent_C|SetHealth _returnvalue_2 (- _output_get (LocalVariables|GetHealth%20To%20Sub))))
  (bind _returnvalue_3 (Class|FunctionalTest|AssertEqualInt _output_get_2 (LocalVariables|GetHealth%20After%20Sub)))
  (return _returnvalue_3))