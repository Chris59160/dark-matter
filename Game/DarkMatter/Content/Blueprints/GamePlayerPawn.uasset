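; Player pawn that routes input to its components for movement, sprinting, light-bullet firing and camera zoom.
; PlayerMovement receives both move axes and switches speed while Sprint is held.
; FireLight starts DoubleShotDirectionComponent shooting from left and right spawn points and flags release; SingleShotDirectionComponent gets a spawn point but is never fired here.
; Zoom plays a timeline forward or in reverse to drive the view-target CameraActor's field of view.
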(event EventBeginPlay
  (Input|EnableInput (Game|GetPlayerController 0))
  (Default|SetLocationComponent (Variables|Default|GetSingleShotDirectionComponent) (Variables|Default|GetSingletBulletSpawnLocation))
  (Default|SetLocationComponent (Variables|Default|GetDoubleShotDirectionComponent) (Variables|Default|GetLeftBulletSpawnLocation) (Variables|Default|GetRightBulletSpawnLocation)))

(event Collision|EventActorBeginOverlap
  (params (OtherActor :type Actor%20Object%20Reference)))

(event EventTick
  (params (DeltaSeconds :type Float%20%28single-precision%29)))

(event Input|ActionEvents|InputActionFireLight
  (params (Key :type Key%20Structure :default "None"))
  (bind _doubleshotdirectioncomponent (Variables|Default|GetDoubleShotDirectionComponent))
  ;[1 1 1] Fire Light Bullet
  (:Pressed
    (Variables|/Game/Components/ShotDirectionComponent.ShotDirectionComponent_C|SetFireShotReleased _doubleshotdirectioncomponent false)
    (Default|StartShooting _doubleshotdirectioncomponent))
  (:Released
    (Variables|/Game/Components/ShotDirectionComponent.ShotDirectionComponent_C|SetFireShotReleased _doubleshotdirectioncomponent true)))

(event Input|ActionEvents|InputActionSprint
  (params (Key :type Key%20Structure :default "None"))
  (bind _playermovement (Variables|Default|GetPlayerMovement))
  ;[1 1 1] Update Speed in PlayerMovement
  (:Pressed
    (Default|SetSpeed _playermovement 1000))
  (:Released
    (Default|SetSpeed _playermovement 500)))

(event Input|ActionEvents|InputActionZoom
  (params (Key :type Key%20Structure :default "None"))
  ;[1 1 1] Zoom In Out In Front of the Camera
  (:Pressed
    (bind _zoom (Timeline|Zoom%20In%20Out Play)
      (:Update
        (bind _ascamera_actor (Utilities|Casting|CastToCameraActor (Pawn|GetViewTarget (Game|GetPlayerController 0))))
        (Camera|SetFieldOfView (Variables|/Script/Engine.CameraActor|GetCameraComponent _ascamera_actor) _zoom))))
  (:Released
    (Timeline|Zoom%20In%20Out Reverse)))

(event Input|AxisEvents|InputAxisMoveLateral
  (params (AxisValue :type Float%20%28single-precision%29))
  ;[1 1 1] Move Lateral managed by PlayerMovement
  (Default|MoveLateral (Variables|Default|GetPlayerMovement) AxisValue))

(event Input|AxisEvents|InputAxisMoveForward
  (params (AxisValue :type Float%20%28single-precision%29))
  ;[1 1 1] Move Forward managed by PlayerMovement
  (Default|MoveForward (Variables|Default|GetPlayerMovement) AxisValue))

(fn ConstructionScript)